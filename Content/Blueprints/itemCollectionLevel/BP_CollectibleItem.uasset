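; A collectible item actor that spins, bobs and is picked up by the collection game character on overlap.
; Tick yaws it by SpinSpeed and adds a sine-based vertical offset each frame, with random jumps in the accumulated time making the bob irregular.
; When its static mesh is overlapped by an actor implementing BPI_CollectionGameChar, it gets the character reference through the interface, calls ItemCollected and destroys itself.
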(event `self.ReceiveTick`
  (params (DeltaSeconds :type "Float (single-precision)"))
  (set `self.ElapsedTime` (+ (+ (`self.ElapsedTime`) (/ (`KismetMathLibrary.Round` (`KismetMathLibrary.RandomFloatInRange` 0.0 1.0)) 2)) DeltaSeconds))
  (`self.K2_AddActorLocalRotation` (`KismetMathLibrary.MakeRotator` 0.0 0.0 (* DeltaSeconds (`self.SpinSpeed`))))
  (`self.K2_AddActorWorldOffset` (`KismetMathLibrary.MakeVector` 0.0 0.0 (* (`KismetMathLibrary.Sin` (/ (`self.ElapsedTime`) (`self.Frequency`))) (`self.Amplitude`)))))

(event `self.StaticMesh.OnComponentBeginOverlap`
  (params (OverlappedComponent :type "PrimitiveComponent Object Reference") (OtherActor :type "Actor Object Reference") (OtherComp :type "PrimitiveComponent Object Reference") (OtherBodyIndex :type Integer) (bFromSweep :type Boolean) (SweepResult :type "HitResult Structure (by ref)"))
  (if (`KismetSystemLibrary.DoesImplementInterface` OtherActor "/Game/Blueprints/Interfaces/BPI_CollectionGameChar.BPI_CollectionGameChar_C")
    (bind _char (message `/Game/Blueprints/Interfaces/BPI_CollectionGameChar.GetCharRef` OtherActor))
    (`/Game/Blueprints/itemCollectionLevel/BP_ItemCollectionChar.ItemCollected` _char)
    (`self.K2_DestroyActor`)))

(fn `UserConstructionScript`)
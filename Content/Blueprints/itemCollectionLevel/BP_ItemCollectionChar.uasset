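; BP_ItemCollectionChar is the character Blueprint for the item collection level, acting as a relay for pickup notifications.
; Its ItemCollected event calls the CollectedItem dispatcher so that bound listeners can react.
; GetCharRef and GetHUDRef expose the character itself and its ItemCollectionHUD reference to other objects.
; BeginPlay and the construction script only call their parents, and Tick and overlap events are disabled.
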(event `self.ReceiveBeginPlay`
  (`parent.ReceiveBeginPlay`))

(event `ItemCollected`
  (`self.CollectedItem`))

(fn `GetCharRef`
  (returns (Char :type "/Game/Blueprints/itemCollectionLevel/BP_ItemCollectionChar Object Reference"))
  (return self))

(fn `GetHUDRef`
  (returns (HUD :type "/Game/Blueprints/Widgets-LevelSpecific/WBP_CollectionLevelHUD Object Reference"))
  (return (`self.ItemCollectionHUD`)))

(fn `UserConstructionScript`
  (`parent.UserConstructionScript`))